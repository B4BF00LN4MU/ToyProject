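; BP_Light1 is a rect light that a linked Switch turns on and off.
; BeginPlay hides the light and binds to the Switch's EventToggle dispatcher, apparently for EventSwitchOverlap, which stores the overlap state in IsPlay.
; Tick sets the light's visibility from IsPlay every frame.
; Disconnected nodes for stepping a relative location along X and Z within bounds never run.
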(event EventBeginPlay
  (Rendering|SetVisibility (Variables|Default|GetRectLight) false false)
  (EventDispatchers|BindEventtoEventDispatcherEventToggle (Variables|Default|GetSwitch) (EventDispatchers|CreateEvent :!event EventSwitchOverlap)))

(event EventTick
  (params (DeltaSeconds :type Float%20%28single-precision%29))
  (bind _rectlight (Variables|Default|GetRectLight))
  (if (Variables|Default|GetIsPlay)
    (Rendering|SetVisibility _rectlight true false)
    (else
      (Rendering|SetVisibility _rectlight false false))))

(fn ConstructionScript)

(fn EventSwitchOverlap
  (params (IsBegin :type Boolean))
  (Variables|Default|SetIsPlay IsBegin))