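; BP_MoveLeftRight1 is an actor that slides its static mesh back and forth along relative X while activated by linked switches.
; BeginPlay binds to the toggle dispatcher of each switch in an array, and an all-switches-on check can set the play flag.
; A separate overlap handler sets that flag directly.
; While active, Tick applies a fixed, frame-rate-dependent step, reversing direction at hard-coded bounds.
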(event EventBeginPlay
  (CallFunction|Bind))

(event EventTick
  (params (DeltaSeconds :type Float%20%28single-precision%29))
  (if (Variables|Default|GetIsPlay)
    (if (Variables|Default|Get오른쪽으로이동하니?)
      ;[1 1 1] 오른쪽으로 이동
      (Variables|Default|SetX에위치 (+ (Variables|Default|GetX에위치) 1.0))
      (Transformation|SetRelativeLocation (Variables|Default|GetStaticMesh) (Math|Vector|MakeVector (Variables|Default|GetX에위치) 0.0 0.0) false false)
      (if (> (Variables|Default|GetX에위치) 2e+02)
        (Variables|Default|Set오른쪽으로이동하니? false))
      (else
        ;[1 1 1] 왼쪽으로 이동
        (Variables|Default|SetX에위치 (+ (Variables|Default|GetX에위치) -1.0))
        (Transformation|SetRelativeLocation (Variables|Default|GetStaticMesh) (Math|Vector|MakeVector (Variables|Default|GetX에위치) 0.0 0.0) false false)
        (if (< (Variables|Default|GetX에위치) 0.0)
          (Variables|Default|Set오른쪽으로이동하니? true))))))

(fn ConstructionScript)

(fn EventSwitchOverlap
  (params (IsBegin :type Boolean))
  (Variables|Default|SetIsPlay IsBegin)
  (return))

(fn Bind
  (for _array_element (Variables|Default|Get조인성)
    (EventDispatchers|BindEventtoEventDispatcherEventToggle _array_element (EventDispatchers|CreateEvent :!event BPMoveLeftRight1AutoGenFunc))))

(fn BPMoveLeftRight1AutoGenFunc
  (params (IsOn :type Boolean))
  (bind _allon (CallFunction|IsAllSwitch))
  (Variables|Default|SetIsPlay _allon))

(fn IsAllSwitch
  (for _array_element (Variables|Default|Get조인성)
    (if (not (Variables|/Game/KyungJun/Blueprints/BP_ToggleSwitch.BP_ToggleSwitch_C|GetIsOn _array_element))
      (return false)))
  (return true))