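; BP_Timer is a stopwatch that shows elapsed minutes and seconds on a text render component.
; On BeginPlay it binds to the overlap dispatcher of a Switch reference, and EventSwitchOverlap sets IsPlay from the begin/end flag.
; While IsPlay is true, Tick accumulates delta time and formats it as zero-padded MM:SS via FloatToStr00; the total is never reset.
; An older, branch-based formatting chain remains disconnected in the EventGraph.
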(event EventBeginPlay
  (EventDispatchers|BindEventtoEventDispatcherOverlap (Variables|Default|GetSwitch) (EventDispatchers|CreateEvent :!event EventSwitchOverlap)))

(event EventTick
  (params (DeltaSeconds :type Float%20%28single-precision%29))
  (if (Variables|Default|GetIsPlay)
    (bind _output_get (Variables|Default|SetTotalDS (+ (Variables|Default|GetTotalDS) DeltaSeconds)))
    (Rendering|Components|TextRender|SetText (Variables|Default|GetTextRender) (Utilities|Text|ToText(String) (Utilities|String|Append (aaa|FloattoStr00 (/ _output_get 6e+01)) ":" (aaa|FloattoStr00 (Math|Float|%(Float) _output_get 6e+01)))))))

(fn ConstructionScript)

(fn FloattoStr00
  (params (Number :type Float%20%28double-precision%29))
  (bind _returnvalue (Math|Float|Floor Number))
  (if (< Number 1e+01)
    (return (Utilities|String|Append "0" (Utilities|String|ToString(Integer) _returnvalue)))
    (else
      (return (Utilities|String|ToString(Integer) _returnvalue)))))

(fn EventSwitchOverlap
  (params (IsBegin :type Boolean))
  (Variables|Default|SetIsPlay IsBegin))