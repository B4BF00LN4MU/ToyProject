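; BP_ToggleSwitch is a switch that flips between on and off whenever something begins overlapping its static mesh.
; DoToggleSwitch inverts IsOn and swaps the mesh material between gold metal when on and a basic wall material when off.
; The overlap event then broadcasts the new state through the EventToggle dispatcher, with no filter on the overlapping actor.
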(event OnComponentBeginOverlap(StaticMesh)
  (params (OverlappedComponent :type Primitive%20Component%20Object%20Reference) (OtherActor :type Actor%20Object%20Reference) (OtherComp :type Primitive%20Component%20Object%20Reference) (OtherBodyIndex :type Integer) (bFromSweep :type Boolean) (SweepResult :type Hit%20Result%20Structure%20%28by%20ref%29))
  (CallFunction|DoToggleSwitch)
  (Default|CallEventDispatcherEventToggle (Variables|Default|GetIsOn)))

(fn ConstructionScript)

(fn DoToggleSwitch
  (bind _staticmesh (Variables|Default|GetStaticMesh))
  (bind _output_get (Variables|Default|SetIsOn (not (Variables|Default|GetIsOn))))
  (if _output_get
    (Rendering|Material|SetMaterial _staticmesh 0 "/Game/StarterContent/Materials/M_Metal_Gold.M_Metal_Gold")
    (else
      (Rendering|Material|SetMaterial _staticmesh 0 "/Game/StarterContent/Materials/M_Basic_Wall.M_Basic_Wall"))))